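; Game mode for a two-team ball game that assigns players to Crimson Corsairs or Cobalt Cavaliers, spawning and possessing their Hexjumper characters.
; Team cap checks redirect overflow joins to the other team.
; Spawns draw random tagged PlayerStarts, removing each from a pool that refills when empty.
; It forwards goals to LobbyGameState and provides events that respawn the ball and return players to team spawns and facings.
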(event `RequestSpawn`
  (params (Team :type "/Game/LobbyBP/Blueprints/Teams Enum" :default "NewEnumerator0") (Controller :type "Controller Object Reference"))
  (bind _returnvalue (`PlayerState.GetPlayerName` (`Controller.PlayerState` Controller)))
  (switch `/Game/LobbyBP/Blueprints/Teams` Team
    (:`NewEnumerator1`
      ;[0 0 0] Run checks to see if teams are full
      (bind _result (`/Engine/EditorBlueprintResources/StandardMacros.IncrementInt` (`self.RedTeamSize`))
        (:`  `
          (if (> (`self.RedTeamSize`) 3)
            (`KismetSystemLibrary.PrintString` "Crimson Corsairs Are Full! Joining Cobalt Cavaliers...")
            (`KismetSystemLibrary.Delay` 3.0)
            ;[0 0 0] Spawn Players!
            (if (== (`KismetArrayLibrary.Array_Length` (`self.AvailabeBlueSpawns`)) 0) :!label _label
              (bind _outactors (`GameplayStatics.GetAllActorsOfClassWithTag` "/Script/Engine.PlayerStart" "Blue"))
              (set `self.AvailabeBlueSpawns` _outactors))
            (if (> (`KismetArrayLibrary.Array_Length` (`self.AvailabeBlueSpawns`)) 0)
              (bind _output_get (set `self.ChosenBlueIndex` (`KismetMathLibrary.RandomIntegerInRange` 0 (- (`KismetArrayLibrary.Array_Length` (`self.AvailabeBlueSpawns`)) 1))))
              (bind _output_get_2 (set `self.ChosenBlueSpawn` (`|GetArrayItem` (`self.AvailabeBlueSpawns`) _output_get)))
              (`KismetArrayLibrary.Array_Remove` (`self.AvailabeBlueSpawns`) (`self.ChosenBlueIndex`))
              (bind _returnvalue_2 (`|SpawnActorFromClass` "/Game/FirstPersonBP/Blueprints/Hexjumper_Blue.Hexjumper_Blue_C" (`self.GetTransform` _output_get_2) "AdjustIfPossibleButAlwaysSpawn" "OverrideRootScale" null Team _returnvalue null null))
              (set `self.NewBlueCharacter` _returnvalue_2)
              (bind _aslobby_player_controller (cast `/Game/LobbyBP/Blueprints/LobbyPlayerController` Controller))
              (`/Game/LobbyBP/Blueprints/LobbyPlayerController.SetInitialControlRotation` :`self` _aslobby_player_controller)
              (`Controller.Possess` Controller (`self.NewBlueCharacter`))
              (`KismetArrayLibrary.Array_AddUnique` (`self.SpawnedBlueCharacter`) (`self.NewBlueCharacter`)))
            (else
              (`KismetSystemLibrary.PrintString` (`KismetStringLibrary.Conv_IntToString` _result))
              (if (== (`KismetArrayLibrary.Array_Length` (`self.AvailableRedSpawns`)) 0) :!label _label_2
                (bind _outactors_2 (`GameplayStatics.GetAllActorsOfClassWithTag` "/Script/Engine.PlayerStart" "Red"))
                (set `self.AvailableRedSpawns` _outactors_2))
              (if (> (`KismetArrayLibrary.Array_Length` (`self.AvailableRedSpawns`)) 0)
                (bind _output_get_3 (set `self.ChosenRedIndex` (`KismetMathLibrary.RandomIntegerInRange` 0 (- (`KismetArrayLibrary.Array_Length` (`self.AvailableRedSpawns`)) 1))))
                (bind _output_get_4 (set `self.ChosenRedSpawn` (`|GetArrayItem` (`self.AvailableRedSpawns`) _output_get_3)))
                (`KismetArrayLibrary.Array_Remove` (`self.AvailableRedSpawns`) (`self.ChosenRedIndex`))
                (bind _returnvalue_3 (`|SpawnActorFromClass` "/Game/FirstPersonBP/Blueprints/Hexjumper_Red.Hexjumper_Red_C" (`self.GetTransform` _output_get_4) "AdjustIfPossibleButAlwaysSpawn" "OverrideRootScale" null Team _returnvalue null null))
                (set `self.NewRedCharacter` _returnvalue_3)
                (bind _aslobby_player_controller_2 (cast `/Game/LobbyBP/Blueprints/LobbyPlayerController` Controller))
                (`/Game/LobbyBP/Blueprints/LobbyPlayerController.SetInitialControlRotation` _aslobby_player_controller_2 (struct :`Yaw` 180.0))
                (`Controller.Possess` Controller (`self.NewRedCharacter`))
                (`KismetArrayLibrary.Array_AddUnique` (`self.SpawnedRedCharacter`) (`self.NewRedCharacter`))))))))
    (:`NewEnumerator2`
      (bind _result_2 (`/Engine/EditorBlueprintResources/StandardMacros.IncrementFloat` (`KismetMathLibrary.Conv_IntToDouble` (`self.BlueTeamSize`)))
        (:`  `
          (if (> (`self.BlueTeamSize`) 3)
            (`KismetSystemLibrary.PrintString` "Cobalt Cavaliers Are Full! Joining Crimson Corsairs...")
            (`KismetSystemLibrary.Delay` 3.0)
            (goto _label_2)
            (else
              (`KismetSystemLibrary.PrintString` (`KismetStringLibrary.Conv_DoubleToString` _result_2))
              (goto _label))))))))

(event `Server_HandleGoal`
  (params (bIsBlueGoal :type Boolean))
  ;[0 1 0] Server Handle Goal
  (bind _aslobby_game_state (cast `/Game/LobbyBP/Blueprints/LobbyGameState` (`GameplayStatics.GetGameState`)))
  (`/Game/LobbyBP/Blueprints/LobbyGameState.ScoreGoal` _aslobby_game_state bIsBlueGoal))

(event `ResetCourt`
  ;[0 1 0] Reset Court after scoring, set scoring to false, then destroy ball
  (bind _aslobby_game_state (cast `/Game/LobbyBP/Blueprints/LobbyGameState` (`GameplayStatics.GetGameState`)))
  (set `/Game/LobbyBP/Blueprints/LobbyGameState.CanScore` false _aslobby_game_state)
  (bind _outactors (`GameplayStatics.GetAllActorsOfClass` "/Game/FirstPersonBP/Blueprints/BoomBall.BoomBall_C"))
  (for _array_element _outactors
    ;[0 1 0] Respawn ball again after scoring
    (`self.K2_DestroyActor` _array_element)
    (`KismetSystemLibrary.Delay` 2.0)
    (bind _outactors_2 (`GameplayStatics.GetAllActorsWithTag` "BallSpawn"))
    (`|SpawnActorFromClass` "/Game/FirstPersonBP/Blueprints/BoomBall.BoomBall_C" (`self.GetTransform` (`|GetArrayItem` _outactors_2)) "Undefined" "OverrideRootScale" null null)
    (bind _aslobby_game_state_2 (cast `/Game/LobbyBP/Blueprints/LobbyGameState` (`GameplayStatics.GetGameState`)))
    (set `/Game/LobbyBP/Blueprints/LobbyGameState.CanScore` true _aslobby_game_state_2)))

(event `ResetAllPlayers`
  ;[0 0 0] Reset players to their spawn after scoring
  (`|ExecutionSequence`
    (:`then_0`
      ;[1 0 0] Reset red spawns after scoring
      (for _array_element (`self.SpawnedRedCharacter`)
        (if (== (`KismetArrayLibrary.Array_Length` (`self.AvailableRedSpawns`)) 0)
          (bind _outactors (`GameplayStatics.GetAllActorsOfClassWithTag` "/Script/Engine.PlayerStart" "Red"))
          (set `self.AvailableRedSpawns` _outactors))
        (if (> (`KismetArrayLibrary.Array_Length` (`self.AvailableRedSpawns`)) 0)
          (bind _output_get (set `self.ChosenRedIndex` (`KismetMathLibrary.RandomIntegerInRange` 0 (- (`KismetArrayLibrary.Array_Length` (`self.AvailableRedSpawns`)) 1))))
          (bind _output_get_2 (set `self.ChosenRedSpawn` (`|GetArrayItem` (`self.AvailableRedSpawns`) _output_get)))
          (`KismetArrayLibrary.Array_Remove` (`self.AvailableRedSpawns`) (`self.ChosenRedIndex`))
          (`KismetSystemLibrary.Delay` 2.0)
          (`self.K2_SetActorTransform` _array_element (`self.GetTransform` _output_get_2) false false)
          (bind _aslobby_player_controller (cast `/Game/LobbyBP/Blueprints/LobbyPlayerController` (`Pawn.GetController` _array_element)))
          (`/Game/LobbyBP/Blueprints/LobbyPlayerController.SetInitialControlRotation` _aslobby_player_controller (struct :`Yaw` 180.0)))))
    (:`then_1`
      ;[0 0.1667 1] Reset blue spawns after scoring
      (for _array_element_2 (`self.SpawnedBlueCharacter`)
        (if (== (`KismetArrayLibrary.Array_Length` (`self.AvailabeBlueSpawns`)) 0)
          (bind _outactors_2 (`GameplayStatics.GetAllActorsOfClassWithTag` "/Script/Engine.PlayerStart" "Blue"))
          (set `self.AvailabeBlueSpawns` _outactors_2))
        (if (> (`KismetArrayLibrary.Array_Length` (`self.AvailabeBlueSpawns`)) 0)
          (bind _output_get_3 (set `self.ChosenBlueIndex` (`KismetMathLibrary.RandomIntegerInRange` 0 (- (`KismetArrayLibrary.Array_Length` (`self.AvailabeBlueSpawns`)) 1))))
          (bind _output_get_4 (set `self.ChosenBlueSpawn` (`|GetArrayItem` (`self.AvailabeBlueSpawns`) _output_get_3)))
          (`KismetArrayLibrary.Array_Remove` (`self.AvailabeBlueSpawns`) (`self.ChosenBlueIndex`))
          (`KismetSystemLibrary.Delay` 2.0)
          (`self.K2_SetActorTransform` _array_element_2 (`self.GetTransform` _output_get_4) false false)
          (bind _aslobby_player_controller_2 (cast `/Game/LobbyBP/Blueprints/LobbyPlayerController` (`Pawn.GetController` _array_element_2)))
          (`/Game/LobbyBP/Blueprints/LobbyPlayerController.SetInitialControlRotation` :`self` _aslobby_player_controller_2))))))

(fn `UserConstructionScript`)