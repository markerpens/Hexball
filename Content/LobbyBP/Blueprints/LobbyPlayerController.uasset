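; Lobby player controller that handles team selection, spawn requests and the match-over screen.
; On BeginPlay the server possesses a LobbyView camera, while the local controller opens the TeamSelection widget with UI-only input.
; TeamSelected registers the team with LobbyGameMode, and ClientBeginMatch forwards to ServerBeginMatch, which requests a spawn using the stored team.
; At match end it blends to a CameraActor, pauses the game and shows W_MatchEnd naming the winners.
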(event `SetInitialControlRotation`
  (params (NewRotation :type "Rotator Structure"))
  ;[0.9387 0.4072 1] Set rotation on client, call on gamemode (so players face proper direction upon spawn
  (`self.SetControlRotation` NewRotation))

(event `self.ReceiveBeginPlay`
  (bind _returnvalue (`GameplayStatics.GetPlayerController` 0))
  (`|ExecutionSequence`
    (:`then_0`
      ;[0 0 0] Possess lobby camera on server
      (`/Engine/EditorBlueprintResources/ActorMacros.Switch Has Authority`
        (:`Authority`
          (bind _outactors (`GameplayStatics.GetAllActorsOfClass` "/Game/LobbyBP/Blueprints/LobbyView.LobbyView_C"))
          (`self.Possess` (`|GetArrayItem` _outactors)))))
    (:`then_1`
      ;[0 0 0] Create widget on local
      (if (`self.IsLocalController`)
        (bind _returnvalue_2 (`|CreateWidget` "/Game/LobbyBP/Blueprints/Widgets/TeamSelection.TeamSelection_C"))
        (`UserWidget.AddToViewport` _returnvalue_2 0)
        (`WidgetBlueprintLibrary.SetInputMode_UIOnlyEx` _returnvalue null)
        (set `PlayerController.bShowMouseCursor` true _returnvalue)))))

(event `ClientBeginMatch`
  (params (Team :type "/Game/LobbyBP/Blueprints/Teams Enum" :default "NewEnumerator0"))
  (`self.ServerBeginMatch` self Team))

(event `TeamSelected`
  (params (`Chosen Team` :type "/Game/LobbyBP/Blueprints/Teams Enum" :default "NewEnumerator0"))
  ;[0 1 0] Select team on server-side
  (set `self.SelectedTeam` `Chosen Team`)
  (`/Game/LobbyBP/Blueprints/LobbyGameMode.RegisterPlayerTeam` (cast `/Game/LobbyBP/Blueprints/LobbyGameMode` (`GameplayStatics.GetGameMode`) :!pure true) self))

(event `ServerBeginMatch`
  (params (Team :type "/Game/LobbyBP/Blueprints/Teams Enum" :default "NewEnumerator0"))
  (`/Game/LobbyBP/Blueprints/LobbyGameMode.RequestSpawn` (cast `/Game/LobbyBP/Blueprints/LobbyGameMode` (`GameplayStatics.GetGameMode`) :!pure true) (`self.SelectedTeam`) self))

(event `Client_ShowMatchEndScreen`
  (params (WinningTeam :type Name))
  ;[0 0 0] Show Match Over to Clients (called in LobbyGameState
  (switch `name` WinningTeam
    (:`Red`
      (bind _outactors (`GameplayStatics.GetAllActorsOfClass` "/Script/Engine.CameraActor"))
      (`self.SetViewTargetWithBlend` (`|GetArrayItem` _outactors) 1.0 "VTBlend_EaseInOut")
      (`GameplayStatics.SetGamePaused` true)
      (bind _returnvalue (`|CreateWidget` "/Game/FirstPersonBP/Blueprints/Widgets/W_MatchEnd.W_MatchEnd_C" (`GameplayStatics.GetPlayerController` 0) "Crimson Corsairs Win!"))
      (`UserWidget.AddToViewport` _returnvalue 0))
    (:`Blue`
      (bind _outactors_2 (`GameplayStatics.GetAllActorsOfClass` "/Script/Engine.CameraActor"))
      (`self.SetViewTargetWithBlend` (`|GetArrayItem` _outactors_2) 2.0 "VTBlend_EaseInOut")
      (`GameplayStatics.SetGamePaused` true)
      (bind _returnvalue_2 (`|CreateWidget` "/Game/FirstPersonBP/Blueprints/Widgets/W_MatchEnd.W_MatchEnd_C" (`GameplayStatics.GetPlayerController` 0) "Cobalt Cavaliers Win!"))
      (`UserWidget.AddToViewport` _returnvalue_2 0))))

(fn `UserConstructionScript`)